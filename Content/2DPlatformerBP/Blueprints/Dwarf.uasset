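; Player dwarf character for a 2D platformer, with movement, jump, crouch, melee attack, health and checkpoint returns that cost damage.
; A function selects the flipbook from movement and action states, refreshed by the horizontal axis event.
; Tick triggers a DoOnce-gated overlap hit check on attack frame 1, applying normal or power damage.
; HUD widgets show damage, key and pickaxe animations; death and win show screens, then reload the map.
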(event `InputAxis|MoveHorizontal`
  (params (AxisValue :type "Float (single-precision)"))
  ;[1 1 1] Rotate Based on Key Press
  (`self.AddMovementInput` (1.0 0.0 0.0) AxisValue)
  (`self.UpdateAnimations`)
  (`/Engine/EditorBlueprintResources/StandardMacros.CompareFloat` AxisValue
    (:`>`
      (`Controller.SetControlRotation` (`self.GetController`) (`KismetMathLibrary.MakeRotator` 0.0))
      (`SceneComponent.K2_SetRelativeRotation` :`self` (`self.Icon`)))
    (:`<`
      (`Controller.SetControlRotation` (`self.GetController`) (`KismetMathLibrary.MakeRotator` 0.0 0.0 180.0))
      (`SceneComponent.K2_SetRelativeRotation` (`self.Icon`) (struct :`Yaw` 180.0) false false))))

(event `DeathScreen`
  ;[0.25 0 1] DeathScreen
  (bind _returnvalue (`|CreateWidget` "/Game/2DPlatformerBP/UI/DeathScreen.DeathScreen_C"))
  (`UserWidget.AddToViewport` _returnvalue 0)
  (`UserWidget.PlayAnimation` _returnvalue (`/Game/2DPlatformerBP/UI/DeathScreen.DeathScreen` _returnvalue) 0.0 1 "Forward" 1.0 false))

(event `ReturnToPreviousCheckpoint`
  ;[1 0.6102 0] Moves the character to the last checkpoint
  (`GameplayStatics.ApplyDamage` self 25.0)
  (`self.K2_SetActorLocation` (`self.CheckpointPos`)))

(event `UpdateAnimations`
  ;[1 0.5237 0.03349] Update Animations
  (bind _selectedanimation (`self.AnimationStateMachine` (`self.IsDown`) (`self.IsAttacking`) (`NavMovementComponent.IsFalling` (`self.CharacterMovement`)) (> (`KismetMathLibrary.VSize` (`self.GetVelocity`)) 0.0) (`NavMovementComponent.IsCrouching` (`self.CharacterMovement`))))
  (`PaperFlipbookComponent.SetFlipbook` (`self.Sprite`) _selectedanimation))

(event `Win`
  ;[1 0.8373 0.09002] PlayerWin
  (`ActorComponent.Deactivate` (`self.CharacterMovement`))
  (`self.DisableInput` null)
  (bind _returnvalue (`|CreateWidget` "/Game/2DPlatformerBP/UI/WinUI.WinUI_C"))
  (`UserWidget.AddToViewport` _returnvalue 0)
  (bind _appear (`/Game/2DPlatformerBP/UI/WinUI.Appear` _returnvalue))
  (`UserWidget.PlayAnimation` _returnvalue _appear 0.0 1 "Forward" 1.0 false)
  (`KismetSystemLibrary.Delay` 10.0)
  (`UserWidget.PlayAnimationReverse` _returnvalue _appear 1.0 false)
  (`GameplayStatics.OpenLevelBySoftObjectPtr` "/Game/2DPlatformerBP/Maps/MainGame_Map.MainGame_Map"))

(event `InputAction|Jump`
  (params (Key :type "Key Structure"))
  ;[0.4022 1 0.5165] Jump Logic
  (:`Pressed`
    (`self.Jump`)))

(event `Down`
  ;[1 0.003866 0] Death Logic
  (set `self.IsDown` true)
  (`self.DeathScreen`)
  (`PaperFlipbookComponent.SetLooping` (`self.Sprite`) false)
  (`PrimitiveComponent.SetCollisionEnabled` (`self.CapsuleComponent`) "NoCollision")
  (`CharacterMovementComponent.DisableMovement` (`self.CharacterMovement`))
  (`KismetSystemLibrary.Delay` 0.1)
  (`self.DisableInput` null)
  (`KismetSystemLibrary.Delay` 6.0)
  (`GameplayStatics.OpenLevelBySoftObjectPtr` "/Game/2DPlatformerBP/Maps/MainGame_Map.MainGame_Map"))

(event `self.OnLanded`
  (params (Hit :type "HitResult Structure (by ref)"))
  ;[0.4022 1 0.5165] Jump Logic
  (`self.StopJumping`))

(event `InputAction|Attack`
  (params (Key :type "Key Structure"))
  ;[1 0.1046 0] Hit Check and logic
  (:`Pressed`
    (set `self.IsAttacking` true)
    (if (`self.IsPowerAttack`)
      (`ActorComponent.Deactivate` (`self.CharacterMovement`)))
    (`KismetSystemLibrary.Delay` 0.5)
    (set `self.IsAttacking` false)
    (`ActorComponent.Activate` (`self.CharacterMovement`) false)
    (goto _label :!via `Reset`)))

(event `InputAction|Crouch`
  (params (Key :type "Key Structure"))
  ;[0.3872 0.4056 1] Crouch Logic
  (:`Pressed`
    (`self.Crouch`))
  (:`Released`
    (`self.UnCrouch`)))

(event `self.ReceiveTick`
  (params (DeltaSeconds :type "Float (single-precision)"))
  ;[1 0.1046 0] Hit Check and logic
  (if (`self.IsAttacking`)
    (if (== (`PaperFlipbookComponent.GetPlaybackPositionInFrames` (`self.Sprite`)) 1)
      (`/Engine/EditorBlueprintResources/StandardMacros.DoOnce` false :!label _label
        (:`Completed`
          (`self.CheckHit`))))))

(event `self.ReceiveAnyDamage`
  (params (Damage :type "Float (single-precision)") (DamageType :type "DamageType Object Reference") (InstigatedBy :type "Controller Object Reference") (DamageCauser :type "Actor Object Reference"))
  ;[1 0.1046 0] Hit Check and logic
  (`UserWidget.PlayAnimation` (stale `self.ReceiveBeginPlay` _returnvalue) (`/Game/2DPlatformerBP/UI/HP.DamageFlash` (stale `self.ReceiveBeginPlay` _returnvalue)) 0.0 1 "Forward" 1.0 false)
  (set `self.Health` (- (`self.Health`) Damage))
  (if (<= (`self.Health`) 0.0)
    (`self.Down`)
    (else
      (`PaperFlipbookComponent.SetSpriteColor` (`self.Sprite`) (struct :`R` 1.0 :`G` 0.1875 :`B` 0.1875 :`A` 1.0))
      (`KismetSystemLibrary.Delay` 0.5)
      (`PaperFlipbookComponent.SetSpriteColor` (`self.Sprite`) (struct :`R` 1.0 :`G` 1.0 :`B` 1.0 :`A` 1.0)))))

(event `self.ReceiveBeginPlay`
  ;[0.3356 0.5439 1] Add UI To Viewport
  (bind _returnvalue (`|CreateWidget` "/Game/2DPlatformerBP/UI/HP.HP_C"))
  (`UserWidget.AddToViewport` _returnvalue 0))

(event `KeyAppear`
  ;[0.3335 0.332 0.3635] Make Key Appear/Disappear
  (`UserWidget.PlayAnimationForward` (stale `self.ReceiveBeginPlay` _returnvalue) (`/Game/2DPlatformerBP/UI/HP.KeyAppear` (stale `self.ReceiveBeginPlay` _returnvalue)) 1.0 false))

(event `KeyDisappear`
  ;[0.3335 0.332 0.3635] Make Key Appear/Disappear
  (`UserWidget.PlayAnimationReverse` (stale `self.ReceiveBeginPlay` _returnvalue) (`/Game/2DPlatformerBP/UI/HP.KeyAppear` (stale `self.ReceiveBeginPlay` _returnvalue)) 1.0 false))

(event `PickaxeAppear`
  ;[0.4927 0.4927 0.4927] Make pickaxe appear/disappear
  (`UserWidget.PlayAnimationForward` (stale `self.ReceiveBeginPlay` _returnvalue) (`/Game/2DPlatformerBP/UI/HP.PickaxeAppear` (stale `self.ReceiveBeginPlay` _returnvalue)) 1.0 false))

(event `PickaxeDisappear`
  ;[0.4927 0.4927 0.4927] Make pickaxe appear/disappear
  (`UserWidget.PlayAnimationReverse` (stale `self.ReceiveBeginPlay` _returnvalue) (`/Game/2DPlatformerBP/UI/HP.PickaxeAppear` (stale `self.ReceiveBeginPlay` _returnvalue)) 1.0 false))

(fn `AnimationStateMachine`
  (params (IsDown :type Boolean) (IsAttacking :type Boolean) (IsFalling :type Boolean) (IsMoving :type Boolean) (IsCrouched :type Boolean))
  (returns (SelectedAnimation :type "PaperFlipbook Object Reference"))
  (if IsDown
    (set `self.States` "NewEnumerator3")
    (elif IsAttacking
      (set `self.States` "NewEnumerator2")
      (elif IsFalling
        (set `self.States` "NewEnumerator4")
        (elif IsMoving
          (set `self.States` "NewEnumerator1")
          (elif IsCrouched
            (set `self.States` "NewEnumerator5")
            (else
              (set `self.States` "NewEnumerator0")))))))
  (return (select `/Game/Assets/Data/CharacterStates` (`self.States`) :`NewEnumerator0` "/Game/Assets/FlipBooks/Dwarf_Idle.Dwarf_Idle" :`NewEnumerator1` "/Game/Assets/FlipBooks/Dwarf_Run.Dwarf_Run" :`NewEnumerator2` "/Game/Assets/FlipBooks/Dwarf_Attack.Dwarf_Attack" :`NewEnumerator3` "/Game/Assets/FlipBooks/Dwarf_Fall.Dwarf_Fall" :`NewEnumerator4` "/Game/Assets/FlipBooks/Dwarf_Jump.Dwarf_Jump" :`NewEnumerator5` "/Game/Assets/FlipBooks/Dwarf_Crouch.Dwarf_Crouch" :!type "PaperFlipbook Object Reference")))

(fn `CheckHit`
  (for _array_element (`PrimitiveComponent.GetOverlappingActors` (`self.AttackHitbox`) "/Script/Engine.Actor")
    (if (!= _array_element self)
      (if (`self.IsPowerAttack`)
        (`GameplayStatics.ApplyDamage` _array_element (`self.Base Power Damage`))
        (else
          (`GameplayStatics.ApplyDamage` _array_element (`self.Base Damage`)))))))

(fn `UserConstructionScript`)