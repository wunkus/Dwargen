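; Goblin King enemy for a 2D platformer that patrols sideways, attacks the Dwarf and drops a Key on death.
; Tick drives movement and picks flipbooks by state; capsule hits either start an attack or reverse direction.
; Attacks pause movement and damage hitbox overlaps once, on animation frame 3, through a DoOnce.
; Damage briefly darkens the sprite, turns it around, swaps the icon at low health, and eventually triggers delayed death.
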(event `Direction`
  (bind _movingright (`self.MovingRight`))
  ;[1 1 1] AI Movement Logic
  (`SceneComponent.K2_SetRelativeRotation` (`self.Icon`) (`KismetMathLibrary.MakeRotator` 0.0 0.0 (select `bool` _movingright :`false` 180.0 :!type "Float (single-precision)")) false false)
  (`self.K2_SetActorRotation` (`KismetMathLibrary.MakeRotator` 0.0 0.0 (select `bool` _movingright :`false` 180.0 :!type "Float (single-precision)")))
  (`self.AddMovementInput` (select `bool` _movingright :`false` (-1.0 0.0 0.0) :`true` (1.0 0.0 0.0) :!type "Vector Structure")))

(event `UpdateAnimations`
  ;[1 0.5237 0.03349] Update Animations
  (bind _selectedanimation (`self.AnimationStateMachine` (`self.IsDown`) (`self.IsAttacking`) (> (`KismetMathLibrary.VSize` (`self.GetVelocity`)) 0.0)))
  (`PaperFlipbookComponent.SetFlipbook` (`self.Sprite`) _selectedanimation))

(event `self.CapsuleComponent.OnComponentHit`
  (params (HitComponent :type "PrimitiveComponent Object Reference") (OtherActor :type "Actor Object Reference") (OtherComp :type "PrimitiveComponent Object Reference") (NormalImpulse :type "Vector Structure") (Hit :type "HitResult Structure (by ref)"))
  ;[0.2864 0.5921 1] Change Direction
  (cast `/Game/2DPlatformerBP/Blueprints/Dwarf` OtherActor
    (:`then`
      (`self.Attack`))
    (:`CastFailed`
      (set `self.MovingRight` (not (`self.MovingRight`))))))

(event `Down`
  ;[1 0.003866 0] Death Logic
  (set `self.IsDown` true)
  (`CharacterMovementComponent.DisableMovement` (`self.CharacterMovement`))
  (`PrimitiveComponent.SetCollisionEnabled` (`self.CapsuleComponent`) "NoCollision")
  (`KismetSystemLibrary.Delay` 6.0)
  (`|SpawnActorFromClass` "/Game/Assets/Blueprints/Key.Key_C" (`KismetMathLibrary.Conv_VectorToTransform` (`self.K2_GetActorLocation`)) "Undefined" "MultiplyWithRoot" null null)
  (`self.K2_DestroyActor`))

(event `Attack`
  ;[1 0.1046 0] Hit Check and logic
  (`ActorComponent.Deactivate` (`self.CharacterMovement`))
  (set `self.IsAttacking` true)
  (`KismetSystemLibrary.Delay` 0.5)
  (set `self.IsAttacking` false)
  (`ActorComponent.Activate` (`self.CharacterMovement`) false)
  (goto _label :!via `Reset`))

(event `self.ReceiveTick`
  (params (DeltaSeconds :type "Float (single-precision)"))
  ;[1 0.1046 0] Hit Check and logic
  (`self.Direction`)
  (`self.UpdateAnimations`)
  (if (`self.IsAttacking`)
    (if (== (`PaperFlipbookComponent.GetPlaybackPositionInFrames` (`self.Sprite`)) 3)
      (`/Engine/EditorBlueprintResources/StandardMacros.DoOnce` false :!label _label
        (:`Completed`
          (`self.CheckHit`))))))

(event `self.ReceiveAnyDamage`
  (params (Damage :type "Float (single-precision)") (DamageType :type "DamageType Object Reference") (InstigatedBy :type "Controller Object Reference") (DamageCauser :type "Actor Object Reference"))
  ;[1 0.1046 0] Hit Check and logic
  (`PaperFlipbookComponent.SetSpriteColor` (`self.Sprite`) (struct :`R` 0.133333 :`A` 1.0))
  (`KismetSystemLibrary.Delay` 0.5)
  (`PaperFlipbookComponent.SetSpriteColor` (`self.Sprite`) (struct :`R` 1.0 :`A` 1.0))
  (set `self.MovingRight` (not (`self.MovingRight`)))
  (set `self.Health` (- (`self.Health`) Damage))
  (if (<= (`self.Health`) 0.0)
    (`SceneComponent.SetVisibility` (`self.Icon`) false false)
    (`self.Down`)
    (elif (<= (`self.Health`) 100.0)
      (`PaperSpriteComponent.SetSprite` (`self.Icon`) "/Game/Assets/Sprites/Enemy/Goblin/Goblin_Sprite_13.Goblin_Sprite_13"))))

(fn `AnimationStateMachine`
  (params (IsDown :type Boolean) (IsAttacking :type Boolean) (IsMoving :type Boolean))
  (returns (SelectedAnimation :type "PaperFlipbook Object Reference"))
  (if IsDown
    (set `self.States` "NewEnumerator3")
    (elif IsAttacking
      (set `self.States` "NewEnumerator2")
      (elif IsMoving
        (set `self.States` "NewEnumerator1")
        (else
          (set `self.States` "NewEnumerator0")))))
  (return (select `/Game/Assets/Data/CharacterStates` (`self.States`) :`NewEnumerator0` "/Game/Assets/FlipBooks/Enemy/Goblin/Goblin_Idle.Goblin_Idle" :`NewEnumerator1` "/Game/Assets/FlipBooks/Enemy/Goblin/Goblin_Run.Goblin_Run" :`NewEnumerator2` "/Game/Assets/FlipBooks/Enemy/Goblin/Goblin_Attack.Goblin_Attack" :`NewEnumerator3` "/Game/Assets/FlipBooks/Enemy/Goblin/GoblinDown.GoblinDown" :!type "PaperFlipbook Object Reference")))

(fn `CheckHit`
  (for _array_element (`PrimitiveComponent.GetOverlappingActors` (`self.AttackHitbox`) "/Script/Engine.Actor")
    (if (!= _array_element self)
      (`GameplayStatics.ApplyDamage` _array_element (`self.Base Damage`)))))

(fn `UserConstructionScript`)