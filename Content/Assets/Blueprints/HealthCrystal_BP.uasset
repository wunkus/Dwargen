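; Health crystal pickup that heals a Dwarf with health below 100 and then destroys itself.
; Logic runs on AnyDamage but casts the OtherActor pin of the otherwise empty ActorBeginOverlap event.
; Healing adds a fixed amount without clamping, then spawns randomly offset debris actors with random lifespans.
; At full health, the crystal stays and shows an animated HealthFull warning widget instead.
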(event `self.ReceiveAnyDamage`
  (params (Damage :type "Float (single-precision)") (DamageType :type "DamageType Object Reference") (InstigatedBy :type "Controller Object Reference") (DamageCauser :type "Actor Object Reference"))
  ;[1 0.01955 0.3044] Heal Player
  (bind _asdwarf (cast `/Game/2DPlatformerBP/Blueprints/Dwarf` (stale `self.ReceiveActorBeginOverlap` OtherActor)))
  (bind _health (`/Game/2DPlatformerBP/Blueprints/Dwarf.Health` _asdwarf))
  (if (< _health 100.0)
    (set `/Game/2DPlatformerBP/Blueprints/Dwarf.Health` (+ _health 20.0) _asdwarf)
    ;[0.6892 0.502 1] Creates a particle effect after crystal is destroyed
    (for _ (range 1 21)
      (bind _returnvalue (`|SpawnActorFromClass` "/Game/Assets/Objects/HealthCrystalDebris.HealthCrystalDebris_C" (`KismetMathLibrary.MakeTransform` (+ (`KismetMathLibrary.MakeVector` (`KismetMathLibrary.RandomFloatInRange` -5.0 5.0) 0.0 (`KismetMathLibrary.RandomFloatInRange` -5.0 5.0)) (`self.K2_GetActorLocation` self))) "Undefined" "MultiplyWithRoot" null null))
      (`self.SetLifeSpan` _returnvalue (`KismetMathLibrary.RandomFloatInRange` 5.0 15.0)))
    (`self.K2_DestroyActor` self)
    (else
      ;[1 0 0] Adds an error message onscreen
      (bind _returnvalue_2 (`|CreateWidget` "/Game/2DPlatformerBP/UI/HealthFull.HealthFull_C"))
      (`UserWidget.AddToViewport` _returnvalue_2 0)
      (`UserWidget.PlayAnimation` _returnvalue_2 (`/Game/2DPlatformerBP/UI/HealthFull.Animation` _returnvalue_2) 0.0 1 "Forward" 1.0 false))))

(event `self.ReceiveActorBeginOverlap`
  (params (OtherActor :type "Actor Object Reference")))

(fn `UserConstructionScript`)