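; LockedDoor is a 2D sprite door that a Dwarf can open with a key and that acts as a checkpoint.
; On box overlap, a Dwarf holding a key loses it, the door swaps to another sprite, and the Dwarf's checkpoint position is updated.
; The trigger box then destroys itself, so unlocking happens only once.
; Without a key, it shows an animated KeyNotification widget instead.
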(event `self.Box.OnComponentBeginOverlap`
  (params (OverlappedComponent :type "PrimitiveComponent Object Reference") (OtherActor :type "Actor Object Reference") (OtherComp :type "PrimitiveComponent Object Reference") (OtherBodyIndex :type Integer) (bFromSweep :type Boolean) (SweepResult :type "HitResult Structure (by ref)"))
  (bind _asdwarf (cast `/Game/2DPlatformerBP/Blueprints/Dwarf` OtherActor))
  ;[1 0.07628 0] Displays an error if player does not have a key
  (if (`/Game/2DPlatformerBP/Blueprints/Dwarf.HasKey` _asdwarf)
    ;[0 1 0.1457] Removes the players key and opens the door
    (set `/Game/2DPlatformerBP/Blueprints/Dwarf.HasKey` false _asdwarf)
    (`PaperSpriteComponent.SetSprite` (`self.Door`) "/Game/Assets/Sprites/Terrain/LockedDoor_Sprite_1.LockedDoor_Sprite_1")
    (`/Game/2DPlatformerBP/Blueprints/Dwarf.KeyDisappear` _asdwarf)
    ;[1 0.8425 0] Sets the players checkpoint position
    (set `/Game/2DPlatformerBP/Blueprints/Dwarf.CheckpointPos` (`SceneComponent.K2_GetComponentLocation` (`self.CheckpointPos`)) _asdwarf)
    (`ActorComponent.K2_DestroyComponent` (`self.Box`))
    (else
      (bind _returnvalue (`|CreateWidget` "/Game/2DPlatformerBP/UI/KeyNotification.KeyNotification_C" (`Pawn.GetLocalViewingPlayerController` _asdwarf)))
      (`UserWidget.AddToViewport` _returnvalue 0)
      (`UserWidget.PlayAnimation` _returnvalue (`/Game/2DPlatformerBP/UI/KeyNotification.AppearDisappear` _returnvalue) 0.0 1 "Forward" 1.0 false))))

(fn `UserConstructionScript`)